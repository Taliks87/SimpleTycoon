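; BP_OfficeQuickMoney is a placeable office building that repeatedly produces coins once placed.
; On placement it shows its progress bar and starts a timed Coin run on the Production component, restarting whenever production finishes.
; A dynamic material instance on the mesh switches its base color between white and dark red to indicate whether placement is allowed.
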(event `self.ReceiveBeginPlay`
  (add `self.OnPlacedBuilding` (delegate `OnPlacedBuilding_Event`))
  ;[1 1 1] Set progress bar visibility
  (`SceneComponent.SetVisibility` (`self.BP_ProdactionProgressBar`) false false)
  ;[1 1 1] Create dynamic material
  (bind _returnvalue (`PrimitiveComponent.CreateDynamicMaterialInstance` (`self.StaticMesh`) 0 "/Game/SimpleTychoon/MaterialLibrary/Debug/MI_BaseInterpMesh_WUV.MI_BaseInterpMesh_WUV" "None"))
  (set `self.Material` _returnvalue))

(event `OnPlacedBuilding_Event`
  (`self.StartCoinProduct`)
  ;[1 1 1] Set progress bar visibility
  (`SceneComponent.SetVisibility` (`self.BP_ProdactionProgressBar`) true false))

(event `self.Production.OnProductionFinished`
  (params (Actor :type "Actor Object Reference") (Product :type "EResourceType Enum" :default "Coin"))
  (`self.StartCoinProduct`))

(event `self.OnCanByPlacedChanged`
  (params (bCanByPlacedFlag :type Boolean))
  (bind _material (`self.Material`))
  ;[1 1 1] Switch color if can/can't by placed
  (if bCanByPlacedFlag
    (`MaterialInstanceDynamic.SetVectorParameterValue` _material "BaseColor" (struct :`R` 1.0 :`G` 1.0 :`B` 1.0 :`A` 1.0))
    (else
      (`MaterialInstanceDynamic.SetVectorParameterValue` _material "BaseColor" (struct :`R` 0.380208 :`B` 0.02243 :`A` 1.0)))))

(fn `StartCoinProduct`
  (`ProductionComponent.StartProduction` (`self.Production`) "Coin" (`self.TimeProduct`)))

(fn `UserConstructionScript`)